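; BP_Unit is a unit actor whose skeletal mesh and animation blueprint follow its UnitType: Warrior, Ranger or Slime.
; The construction script applies the matching mesh and anim class.
; From BeginPlay, an endless delay loop cycles a test index through five animation states, sending each to the anim instance via SetUnitAnimationStateMessage, apparently as an animation test.
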(event EventBeginPlay
  (Utilities|FlowControl|Delay 3.0 :!label _label)
  (bind _output_get (Variables|Default|SetTest_AnimIndex (Utilities|Enum|ByteToEnumE_UnitAnimationState (Class|KismetMathLibrary|PercentByteByte (+ (Variables|Default|GetTest_AnimIndex) 1) 5))))
  (Class|BPIUnitAnimation|SetUnitAnimationState(Message) (Components|SkeletalMesh|GetAnimInstance (Variables|Default|GetSkeletalMesh)) _output_get)
  (goto _label))

(fn ConstructionScript
  (Class|SkinnedMeshComponent|SetSkeletalMesh (Variables|Default|GetSkeletalMesh) (Utilities|Select :Index (Variables|Default|GetUnitType) :NewEnumerator0 "/Game/Art/Units/Warrior/SK_Warrior.SK_Warrior" :NewEnumerator1 "/Game/Art/Units/Ranger/SK_Ranger.SK_Ranger" :NewEnumerator2 "/Game/Art/Units/Slime/SK_Slime.SK_Slime") true)
  (Class|SkeletalMeshComponent|SetAnimClass (Variables|Default|GetSkeletalMesh) (Utilities|Select :Index (Variables|Default|GetUnitType) :NewEnumerator0 "/Game/Art/Units/Warrior/ABP_Warrior.ABP_Warrior_C" :NewEnumerator1 "/Game/Art/Units/Ranger/ABP_Ranger.ABP_Ranger_C" :NewEnumerator2 "/Game/Art/Units/Slime/ABP_Slime.ABP_Slime_C")))