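; Grid actor that builds a flat tile grid of squares, hexagons or triangles as instances of one InstancedStaticMesh.
; SpawnGrid clears old tiles, takes mesh, material and size from DT_GridShapeData, then snaps center and bottom-left corner per shape.
; Index-to-transform helpers place each tile, using doubled row indices for hexagons and parity-based yaw flips for triangles.
; Nothing here triggers spawning: events are empty and the construction script's SpawnGrid call is disconnected.
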(event EventBeginPlay)

(event Collision|EventActorBeginOverlap
  (params (OtherActor :type Actor%20Object%20Reference)))

(event EventTick
  (params (DeltaSeconds :type Float%20%28single-precision%29)))

(fn ConstructionScript)

(fn SpawnGrid
  (params (CenterLocation :type Vector) (TileSize :type Vector) (TileCount :type Vector%202D%20Structure) (Shape :type E_GridShapes%20Enum :default "NewEnumerator0"))
  (bind _returnvalue (CallFunction|GetCurrentShapeData))
  (bind _instancedstaticmesh (Variables|Default|GetInstancedStaticMesh))
  (bind (_meshsize _mesh _meshmaterial _flatmesh _flatbordermaterial) (Utilities|Struct|BreakS_GridShapeData _returnvalue))
  (Variables|Default|SetGrid%20Center%20Location CenterLocation)
  (Variables|Default|SetGrid%20Tile%20Size TileSize)
  (Variables|Default|SetGrid%20Shape Shape)
  (Variables|Default|SetGrid%20Tile%20Count (Math|Vector2D|MakeVector2D (Math|Conversions|ToFloat(Integer) (Math|Float|Round (.x TileCount))) (Math|Conversions|ToFloat(Integer) (Math|Float|Round (.y TileCount)))))
  (CallFunction|DestroyGrid)
  (Components|StaticMesh|SetStaticMesh _instancedstaticmesh _flatmesh)
  (Rendering|Material|SetMaterial _instancedstaticmesh 0 _flatbordermaterial)
  (bind (_center _bottomleft) (CallFunction|CalculateCenterandBottomLeft))
  (Variables|Default|SetGrid%20Center%20Location _center)
  (Variables|Default|SetGridBottomLeftCornerLocation _bottomleft)
  (for _index (range 0 (- (Math|Float|Round (.x (Variables|Default|GetGrid%20Tile%20Count))) 1))
    (LocalVariables|SetX _index)
    (if (Utilities|Enum|NotEqual(Enum) (Variables|Default|GetGrid%20Shape) "NewEnumerator2")
      (for _index_2 (range 0 (- (Math|Float|Round (.y (Variables|Default|GetGrid%20Tile%20Count))) 1))
        (LocalVariables|SetY _index_2)
        (LocalVariables|SetIndex (Math|Vector2D|MakeVector2D (Math|Conversions|ToFloat(Integer) (LocalVariables|GetX)) (Math|Conversions|ToFloat(Integer) (LocalVariables|GetY))))
        (LocalVariables|SetTileTransform (Math|Transform|MakeTransform (+ (CallFunction|GetTileLocationfromGridIndex (LocalVariables|GetIndex)) "0, 0,2.000000") (CallFunction|GetTileRotationfromGridIndex (LocalVariables|GetIndex)) (/ (Variables|Default|GetGrid%20Tile%20Size) (.MeshSize (Utilities|Struct|BreakS_GridShapeData (CallFunction|GetCurrentShapeData))))))
        (Class|InstancedStaticMeshComponent|AddInstanceWorldSpace (Variables|Default|GetInstancedStaticMesh) (LocalVariables|GetTileTransform)))
      (else
        (for _index_3 (range (Math|Integer|SelectInt 0 1 (CallFunction|IsIntEven (LocalVariables|GetX))) (- (* (Math|Float|Round (.y (Variables|Default|GetGrid%20Tile%20Count))) 2) 1))
          (LocalVariables|SetY _index_3)
          (Utilities|FlowControl|Sequence
            (:then_0
              (LocalVariables|SetIndex (Math|Vector2D|MakeVector2D (Math|Conversions|ToFloat(Integer) (LocalVariables|GetX)) (Math|Conversions|ToFloat(Integer) (LocalVariables|GetY))))
              (LocalVariables|SetTileTransform (Math|Transform|MakeTransform (+ (CallFunction|GetTileLocationfromGridIndex (LocalVariables|GetIndex)) "0, 0,2.000000") (CallFunction|GetTileRotationfromGridIndex (LocalVariables|GetIndex)) (/ (Variables|Default|GetGrid%20Tile%20Size) (.MeshSize (Utilities|Struct|BreakS_GridShapeData (CallFunction|GetCurrentShapeData))))))
              (Class|InstancedStaticMeshComponent|AddInstanceWorldSpace (Variables|Default|GetInstancedStaticMesh) (LocalVariables|GetTileTransform)))
            (:then_1
              (Math|Integer|IncrementInt _index_3))))))))

(fn GetCurrentShapeData
  (bind _returnvalue (Utilities|GetDataTableRow "/Game/Blueprints/Core/Grid/GridShapes/DT_GridShapeData.DT_GridShapeData" (Utilities|String|StringToName (Utilities|String|EnumtoString (Variables|Default|GetGrid%20Shape))))
    (:then
      (return _returnvalue))))

(fn DestroyGrid
  (Components|InstancedStaticMesh|ClearInstances (Variables|Default|GetInstancedStaticMesh)))

(fn CalculateCenterandBottomLeft
  (bind _grid_tile_count (Variables|Default|GetGrid%20Tile%20Count))
  (switch Utilities|FlowControl|Switch|SwitchonE_GridShapes (Variables|Default|GetGrid%20Shape)
    (:NewEnumerator1
      (LocalVariables|SetC (CallFunction|SnapVectortoVector (Variables|Default|GetGrid%20Center%20Location) (Variables|Default|GetGrid%20Tile%20Size)))
      (return (LocalVariables|GetC) (- (LocalVariables|GetC) (Math|Conversions|ToVector(Vector2D) (* (Math|Conversions|ToVector2D(Vector) (Variables|Default|GetGrid%20Tile%20Size)) (/ (- (Variables|Default|GetGrid%20Tile%20Count) (Math|Vector2D|MakeVector2D (Math|Float|SelectFloat 0.0 1.0 (CallFunction|IsFloatEven (.x _grid_tile_count))) (Math|Float|SelectFloat 0.0 1.0 (CallFunction|IsFloatEven (.y _grid_tile_count))))) 2.0))))))
    (:NewEnumerator2
      (LocalVariables|SetC (CallFunction|SnapVectortoVector (Variables|Default|GetGrid%20Center%20Location) (* (Variables|Default|GetGrid%20Tile%20Size) "1.500000,1.000000,1.000000")))
      (return (LocalVariables|GetC) (- (LocalVariables|GetC) (CallFunction|SnapVectortoVector (Math|Conversions|ToVector(Vector2D) (* (Math|Conversions|ToVector2D(Vector) (Variables|Default|GetGrid%20Tile%20Size)) (/ (Variables|Default|GetGrid%20Tile%20Count) "(X=3.000000,Y=2.000000)"))) (* (Variables|Default|GetGrid%20Tile%20Size) "1.500000,1.000000,1.000000")))))
    (:NewEnumerator3
      (LocalVariables|SetC (CallFunction|SnapVectortoVector (Variables|Default|GetGrid%20Center%20Location) (* (Variables|Default|GetGrid%20Tile%20Size) "2.000000,1.000000,1.000000")))
      (return (LocalVariables|GetC) (- (LocalVariables|GetC) (CallFunction|SnapVectortoVector (Math|Conversions|ToVector(Vector2D) (* (Math|Conversions|ToVector2D(Vector) (Variables|Default|GetGrid%20Tile%20Size)) (/ (- (Variables|Default|GetGrid%20Tile%20Count) (Math|Vector2D|MakeVector2D 1.0 1.0)) "(X=2.000000,Y=4.000000)"))) (* (Variables|Default|GetGrid%20Tile%20Size) "2.000000,1.000000,1.000000")))))))

(fn GetTileRotationfromGridIndex
  (params (GridIndex :type Vector%202D%20Structure))
  (if (Utilities|Enum|Equal(Enum) (Variables|Default|GetGrid%20Shape) "NewEnumerator3")
    (return (Math|Rotator|MakeRotator 0.0 0.0 (+ (Math|Float|SelectFloat 1.8e+02 0.0 (CallFunction|IsFloatEven (.x GridIndex))) (Math|Float|SelectFloat 1.8e+02 0.0 (CallFunction|IsFloatEven (.y GridIndex))))))
    (else
      (return "0, 0, 0"))))

(fn GetTileLocationfromGridIndex
  (params (GridIndex :type Vector%202D%20Structure))
  (return (+ (Variables|Default|GetGridBottomLeftCornerLocation) (* (Variables|Default|GetGrid%20Tile%20Size) (Math|Conversions|ToVector(Vector2D) (* GridIndex (Utilities|Select :Index (Variables|Default|GetGrid%20Shape) :NewEnumerator0 "" :NewEnumerator1 "(X=1.000000,Y=1.000000)" :NewEnumerator2 "(X=0.750000,Y=0.500000)" :NewEnumerator3 "(X=1.000000,Y=0.500000)")))))))