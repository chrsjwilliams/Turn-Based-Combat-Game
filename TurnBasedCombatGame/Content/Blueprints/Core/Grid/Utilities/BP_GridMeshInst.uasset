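; BP_GridMeshInst is a grid utility actor that renders tiles as instances of one configurable mesh, colored by tile state.
; A parallel index array maps grid indices to instance slots, so tiles can be replaced, removed or cleared.
; AddInstance writes the highest-priority state's color and a filled flag into per-instance custom data for the material.
; InitializeMeshInst sets mesh, material, base color and collision, and actor tick is disabled at BeginPlay.
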(event EventBeginPlay
  (Actor|Tick|SetActorTickEnabled false))

(event Collision|EventActorBeginOverlap
  (params (OtherActor :type Actor%20Object%20Reference)))

(event EventTick
  (params (DeltaSeconds :type Float%20%28single-precision%29)))

(fn ConstructionScript)

(fn AddInstance
  (params (Index :type Int%20Point%20Structure%20%28by%20ref%29) (Transform :type Transform%20%28by%20ref%29) (States :type Array%20of%20E_TileState%20Enums :default "NewEnumerator0"))
  (bind _instancedstaticmesh (Variables|Default|GetInstancedStaticMesh))
  (CallFunction|RemoveInstance Index)
  (Components|InstancedStaticMesh|AddInstance (Variables|Default|GetInstancedStaticMesh) Transform)
  (bind _returnvalue (Utilities|Array|Add (Variables|Default|GetInstanceIndicies) Index))
  (LocalVariables|Seti _returnvalue)
  (bind (_color _isfilled) (CallFunction|GetColorfromStates States))
  (Components|InstancedStaticMesh|SetCustomDataValue _instancedstaticmesh (LocalVariables|Geti) 0 (.R (Math|Color|BreakColor _color)) false)
  (Components|InstancedStaticMesh|SetCustomDataValue _instancedstaticmesh (LocalVariables|Geti) 1 (.G (Math|Color|BreakColor _color)) false)
  (Components|InstancedStaticMesh|SetCustomDataValue _instancedstaticmesh (LocalVariables|Geti) 2 (.B (Math|Color|BreakColor _color)) false)
  (Components|InstancedStaticMesh|SetCustomDataValue _instancedstaticmesh (LocalVariables|Geti) 3 _isfilled false))

(fn RemoveInstance
  (params (Index :type Int%20Point%20Structure%20%28by%20ref%29))
  (bind _instanceindicies (Variables|Default|GetInstanceIndicies))
  (if (Utilities|Array|ContainsItem _instanceindicies Index)
    (Class|InstancedStaticMeshComponent|RemoveInstance (Variables|Default|GetInstancedStaticMesh) (Utilities|Array|FindItem _instanceindicies Index))
    (Utilities|Array|RemoveItem (Variables|Default|GetInstanceIndicies) Index)))

(fn ClearInstances
  (Components|InstancedStaticMesh|ClearInstances (Variables|Default|GetInstancedStaticMesh))
  (Utilities|Array|Clear (Variables|Default|GetInstanceIndicies)))

(fn InitializeMeshInst
  (params (Mesh :type Static%20Mesh%20Object%20Reference) (Material :type Material%20Interface%20Object%20Reference) (inLinearColor :type Linear%20Color%20Structure) (Collision :type ECollisionEnabled%20Enum :default "NoCollision"))
  (bind _instancedstaticmesh (Variables|Default|GetInstancedStaticMesh))
  (Components|StaticMesh|SetStaticMesh _instancedstaticmesh Mesh)
  (Rendering|Material|SetMaterial _instancedstaticmesh 0 Material)
  (Rendering|Material|SetVectorParameterValueonMaterials _instancedstaticmesh "Color" (Math|Conversions|ToVector(LinearColor) inLinearColor))
  (Collision|SetCollisionEnabled _instancedstaticmesh Collision))

(fn GetColorfromStates
  (params (States :type Array%20of%20E_TileState%20Enums :default "NewEnumerator0"))
  (if (== (Utilities|Array|Length States) 0)
    (return "(R=0.000000,G=0.000000,B=0.000000,A=1.000000)" 0.0)
    (else
      (for _array_element (Utilities|Array|MakeArray "NewEnumerator2" "NewEnumerator1" "NewEnumerator3" "NewEnumerator4" "NewEnumerator5" "NewEnumerator6")
        (if (Utilities|Array|ContainsItem States _array_element)
          (return (Utilities|Select :Index _array_element :NewEnumerator0 "" :NewEnumerator1 "(R=1.000000,G=0.233956,B=0.000000,A=1.000000)" :NewEnumerator2 "(R=0.000000,G=0.877233,B=1.000000,A=1.000000)" :NewEnumerator3 "(R=1.000000,G=0.274780,B=0.861326,A=1.000000)" :NewEnumerator4 "(R=0.020301,G=0.000000,B=1.000000,A=1.000000)" :NewEnumerator5 "(R=1.000000,G=0.064580,B=0.000000,A=1.000000)" :NewEnumerator6 "(R=0.514669,G=0.032506,B=0.015884,A=1.000000)") 1.0)))
      (return "(R=0.000000,G=0.000000,B=0.000000,A=1.000000)" 0.0))))