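; BP_GridPathfinding supplies tile adjacency queries for a grid, returning neighbor indexes and filtering them to traversable tiles.
; GetNeighborIndexes dispatches on the grid's shape to fixed offsets for square, hexagon or triangle, with optional diagonals for square and triangle.
; Hexagons use doubled-row offsets, and triangles flip their sideways neighbor by index parity.
; GetValidTileNeighbors keeps only walkable tiles whose height difference is within one tile height; no path search exists yet.
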(event EventBeginPlay)

(event Collision|EventActorBeginOverlap
  (params (OtherActor :type Actor%20Object%20Reference)))

(event EventTick
  (params (DeltaSeconds :type Float%20%28single-precision%29)))

(fn ConstructionScript)

(fn GetNeighborIndexes
  (params (Index :type Int%20Point%20Structure) (IncludeDiagonals :type Boolean))
  (switch Utilities|FlowControl|Switch|SwitchonE_GridShapes (Variables|/Game/Blueprints/Core/Grid/BP_Grid.BP_Grid_C|GetGrid%20Shape (Variables|Default|GetGrid))
    (:NewEnumerator1
      (return (CallFunction|GetNeighborIndexsforSquare Index IncludeDiagonals)))
    (:NewEnumerator2
      (return (CallFunction|GetNeighborIndexesforHexagon Index)))
    (:NewEnumerator3
      (return (CallFunction|GetNeighborIndexesforTriangle Index IncludeDiagonals)))))

(fn GetNeighborIndexsforSquare
  (params (Index :type Int%20Point%20Structure) (IncludeDiagonals :type Boolean))
  (bind _intpoint (Utilities|Struct|MakeIntPoint 1 0))
  (bind _intpoint_2 (Utilities|Struct|MakeIntPoint 0 1))
  (bind _intpoint_3 (Utilities|Struct|MakeIntPoint -1 0))
  (bind _intpoint_4 (Utilities|Struct|MakeIntPoint 0 -1))
  (bind _returnvalue (+ Index _intpoint))
  (bind _returnvalue_2 (+ Index _intpoint_2))
  (bind _returnvalue_3 (+ Index _intpoint_3))
  (bind _returnvalue_4 (+ Index _intpoint_4))
  (bind _array (Utilities|Array|MakeArray _returnvalue _returnvalue_2 _returnvalue_3 _returnvalue_4))
  (if IncludeDiagonals
    (bind _output_get (Variables|Default|SetoutIndexs _array))
    (Utilities|Array|AppendArray _output_get (Utilities|Array|MakeArray (+ Index (Utilities|Struct|MakeIntPoint 1 1)) (+ Index (Utilities|Struct|MakeIntPoint -1 1)) (+ Index (Utilities|Struct|MakeIntPoint 1 -1)) (+ Index (Utilities|Struct|MakeIntPoint -1 -1))))
    (return (Variables|Default|GetoutIndexs))
    (else
      (return _array))))

(fn GetNeighborIndexesforHexagon
  (params (Index :type Int%20Point%20Structure))
  (return (Utilities|Array|MakeArray (+ Index (Utilities|Struct|MakeIntPoint 1 1)) (+ Index (Utilities|Struct|MakeIntPoint 0 2)) (+ Index (Utilities|Struct|MakeIntPoint -1 1)) (+ Index (Utilities|Struct|MakeIntPoint -1 -1)) (+ Index (Utilities|Struct|MakeIntPoint 0 -2)) (+ Index (Utilities|Struct|MakeIntPoint 1 -1)))))

(fn GetNeighborIndexesforTriangle
  (params (Index :type Int%20Point%20Structure) (IncludeDiagonals :type Boolean))
  (LocalVariables|SetoutIndexes (Utilities|Array|MakeArray (+ Index (Utilities|Struct|MakeIntPoint 0 -1)) (+ Index (Utilities|Struct|MakeIntPoint 0 1))))
  (if (Math|Boolean|Equal(Boolean) (CallFunction|IsIntEven (.x Index)) (CallFunction|IsIntEven (.y Index)))
    (Utilities|Array|Add (LocalVariables|GetoutIndexes) (+ Index (Utilities|Struct|MakeIntPoint -1 0)))
    (else
      (Utilities|Array|Add (LocalVariables|GetoutIndexes) (+ Index (Utilities|Struct|MakeIntPoint 1 0)))))
  (if IncludeDiagonals
    (if (Math|Boolean|Equal(Boolean) (CallFunction|IsIntEven (.x Index)) (CallFunction|IsIntEven (.y Index)))
      (Utilities|Array|AppendArray (LocalVariables|GetoutIndexes) (Utilities|Array|MakeArray (+ Index (Utilities|Struct|MakeIntPoint 1 0)) (+ Index (Utilities|Struct|MakeIntPoint -1 2)) (+ Index (Utilities|Struct|MakeIntPoint -1 -2))))
      (else
        (Utilities|Array|AppendArray (LocalVariables|GetoutIndexes) (Utilities|Array|MakeArray (+ Index (Utilities|Struct|MakeIntPoint -1 0)) (+ Index (Utilities|Struct|MakeIntPoint 1 2)) (+ Index (Utilities|Struct|MakeIntPoint 1 -2))))))
    (return (LocalVariables|GetoutIndexes))
    (else
      (return (LocalVariables|GetoutIndexes)))))

(fn GetValidTileNeighbors
  (params (Index :type Int%20Point%20Structure) (IncludeDiagonals :type Boolean))
  (LocalVariables|SetInputData (.Value (Utilities|Map|Find (Variables|/Game/Blueprints/Core/Grid/BP_Grid.BP_Grid_C|GetGridTiles (Variables|Default|GetGrid)) Index)))
  (bind _neighbors (CallFunction|GetNeighborIndexes Index IncludeDiagonals))
  (for _array_element _neighbors
    (LocalVariables|SetData (.Value (Utilities|Map|Find (Variables|/Game/Blueprints/Core/Grid/BP_Grid.BP_Grid_C|GetGridTiles (Variables|Default|GetGrid)) _array_element)))
    (if (CallFunction|IsTileTypeWalkable (.type (LocalVariables|GetData)))
      (if (<= (Math|Float|Absolute(Float) (- (.z (.location (.transform (LocalVariables|GetData)))) (.z (.location (.transform (LocalVariables|GetInputData)))))) (.z (Variables|/Game/Blueprints/Core/Grid/BP_Grid.BP_Grid_C|GetGrid%20Tile%20Size (Variables|Default|GetGrid))))
        (Utilities|Array|Add (LocalVariables|GetoutIndexes) (.index (LocalVariables|GetData))))))
  (return (LocalVariables|GetoutIndexes)))